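; EventTracker component that gates in-game events so they progress in numbered order.
; Progress compares its event number to EventTrack on the GameVariables game instance, advancing it and calling Tracked on a match, or FailedAudio otherwise.
; Event zero calls NonTracked unless TriggerNext is set.
; After each match, it calls TriggerNext on the EventTracker of every actor tagged Triggerable, allowing events to chain.
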(fn Progress
  (params (EventNumber :type Integer) (TriggerNext :type Boolean))
  ;[1 1 1] Checks Whether Objkect is Not Event Tracked, Event Tracked, Or Failed to be next Event
  ;[1 1 1] Performs if Triggered by Previous Event
  (if TriggerNext
    (bind _asgame_variables (Utilities|Casting|CastToGameVariables (Game|GetGameInstance)))
    (if (== (Variables|/Game/Blueprints/GameVariables.GameVariables_C|GetEventTrack _asgame_variables) EventNumber)
      (Default|ProgressEvent _asgame_variables)
      (Default|CallTracked)
      (bind _outactors (Actor|GetAllActorswithTag "Triggerable"))
      (for (_ _array_index) _outactors
        (Default|CallTriggerNext (Actor|GetComponentbyClass (Utilities|Array|Get(acopy) _outactors _array_index) "EventTracker_C")))
      (else
        (Default|CallFailedAudio)))
    (elif (== EventNumber 0)
      (Default|CallNon-Tracked)
      (else
        (bind _asgame_variables_2 (Utilities|Casting|CastToGameVariables (Game|GetGameInstance)))
        (if (== (Variables|/Game/Blueprints/GameVariables.GameVariables_C|GetEventTrack _asgame_variables_2) EventNumber)
          (Default|ProgressEvent _asgame_variables_2)
          (Default|CallTracked)
          (bind _outactors_2 (Actor|GetAllActorswithTag "Triggerable"))
          (for (_ _array_index_2) _outactors_2
            (Default|CallTriggerNext (Actor|GetComponentbyClass (Utilities|Array|Get(acopy) _outactors_2 _array_index_2) "EventTracker_C")))
          (else
            (Default|CallFailedAudio)))))))