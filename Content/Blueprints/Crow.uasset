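; Crow actor that plays a media source and drifts across the scene as a self-replacing ambient bird.
; On BeginPlay it starts the media player and moves its Plane component along negative Y by a random distance over a random time, then spawns a replacement Crow at a randomized position and destroys itself.
; The Caw event is written to call itself, replaying the audio after random delays.
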(event Custom|Caw
  (Utilities|FlowControl|Delay (Math|Random|RandomFloatinRange 5.0 1e+01))
  (Audio|Components|Audio|Play (Variables|Default|GetAudio) 0.0)
  (CallFunction|Caw))

(event EventBeginPlay
  (bind _self self)
  (bind _crow (Variables|Default|GetCrow))
  (bind _returnvalue (Transformation|GetActorLocation _self))
  (Media|MediaPlayer|OpenSource _crow "/Game/Movies/Crow.Crow")
  (Media|MediaPlayer|Play _crow :!class /Script/MediaAssets.MediaPlayer)
  (CallFunction|Caw)
  (Components|MoveComponentTo (Variables|Default|GetPlane) (Math|Vector|MakeVector (.x _returnvalue) (+ (.y _returnvalue) (Math|Random|RandomFloatinRange -5e+02 -2.5e+03)) (.z _returnvalue)) "0.000000,90.000000,90.000000" false false (Math|Random|RandomFloatinRange 7.0 12.0) false)
  (Game|SpawnActorfromClass "Crow_C" (Math|Transform|MakeTransform (Math|Vector|MakeVector 3.5e+02 (Math|Random|RandomFloatinRange -5e+02 -2.5e+03) (Math|Random|RandomFloatinRange 3.5e+02 7.5e+02)) "0.000000,90.000000,90.000000" "1.000000,1.000000,1.000000") "Undefined" "MultiplyWithRoot" 0 0)
  (Actor|DestroyActor))

(fn ConstructionScript)