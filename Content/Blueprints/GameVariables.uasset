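; GameVariables holds player and progress state to carry between levels, including the current level name for saving.
; StoreVariables copies health, radiation, ammo, speed and night vision from the Player actor found by class.
; Separate events record the level name, count key items up to a cap and advance an event progress counter.
; Both counters print debug messages, and the fourth key item message is unreachable under the cap.
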(event Custom|ProgressEvent
  ;[1 1 1] Store Level Progress
  (bind _output_get (Variables|Default|SetEventTrack (+ (Variables|Default|GetEventTrack) 1)))
  (Development|PrintString (Utilities|String|ToString(Integer) _output_get)))

(event Custom|EffectKeyItem
  ;[1 1 1] Add Key Items to Inventory
  (if (< (Variables|Default|GetKeyItems) 3)
    (bind _output_get (Variables|Default|SetKeyItems (+ (Variables|Default|GetKeyItems) 1)))
    (if (== _output_get 1)
      (Development|PrintString "Got One")
      (elif (== _output_get 2)
        (Development|PrintString "Got Two")
        (elif (== _output_get 3)
          (Development|PrintString "Got Three")
          (elif (== _output_get 4)
            (Development|PrintString "Got Four")))))))

(event Custom|StoreVariables
  ;[1 1 1] For Storing Variables Between Levels
  (bind _returnvalue (Actor|GetActorOfClass "/Game/Characters/Player.Player_C"))
  (Variables|Default|SetHealth (Variables|/Game/Characters/Player.Player_C|GetHealth _returnvalue))
  (Variables|Default|SetRadiation (Variables|/Game/Characters/Player.Player_C|GetRadiation _returnvalue))
  (Variables|Default|SetAmmo (Variables|/Game/Characters/Player.Player_C|GetAmmo _returnvalue))
  (Variables|Default|SetSpeed (Variables|/Game/Characters/Player.Player_C|GetSpeed _returnvalue))
  (Variables|Default|SetNightVis (Variables|/Game/Characters/Player.Player_C|GetNightVis _returnvalue)))

(event Custom|StoreLevel
  ;[1 1 1] Store Current Level for Saving
  (bind _returnvalue (Game|GetCurrentLevelName true))
  (Variables|Default|SetCurrentLevel (Utilities|String|StringToName _returnvalue)))